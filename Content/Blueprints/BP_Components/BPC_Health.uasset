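; Health component that tracks current health and alive state for its owner, starting at maximum health on BeginPlay.
; OnChangeHealth applies a signed change only while vulnerable, clamps the result, and clears IsAlive at zero.
; Any accepted change that leaves health above zero, healing included, starts a timed invulnerability window that blocks further changes until ResetVuln fires.
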(event Custom|OnChangeHealth
  (params (HealthChange :type Float%20%28single-precision%29))
  (if (Variables|Default|GetbIsVulnerable)
    (bind _output_get (Variables|Default|SetCurrentHealth (Math|Float|Clamp(Float) (+ (Variables|Default|GetCurrentHealth) HealthChange) 0.0 (Variables|Default|GetMaxHealth))))
    (if (<= _output_get 0.0)
      (Variables|Default|SetbIsAlive false)
      (else
        (Variables|Default|SetbIsVulnerable false)
        (Utilities|Time|SetTimerbyEvent (delegate Custom|ResetVuln) (Variables|Default|GetDamageInvulnTimer))))))

(event Custom|ResetVuln
  (Variables|Default|SetbIsVulnerable true))

(event EventBeginPlay
  (Variables|Default|SetCurrentHealth (Variables|Default|GetMaxHealth)))