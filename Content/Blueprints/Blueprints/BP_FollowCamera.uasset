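; BP_FollowCamera is a camera-follow actor that moves to the first player's pawn location every tick.
; Tick snaps it to the result of FindMovementLocation without interpolation, clamping X and Y to non-negative values within a large upper bound while Z passes through.
; FindMovementLocation branches on the player count from the BP_GameMode cached at BeginPlay, but both branches are empty, so it always returns player 0's location.
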(event EventBeginPlay
  (bind _asbp_game_mode (Utilities|Casting|CastToBP_GameMode (Game|GetGameMode)))
  (Variables|Default|SetGameMode _asbp_game_mode))

(event Collision|EventActorBeginOverlap
  (params (OtherActor :type Actor%20Object%20Reference)))

(event EventTick
  (params (DeltaSeconds :type Float%20%28single-precision%29))
  (bind _movetolocation (CallFunction|FindMovementLocation))
  (Transformation|SetActorLocation (Math|Vector|MakeVector (Math|Float|Clamp(Float) (.x _movetolocation) 0.0 99999.0) (Math|Float|Clamp(Float) (.y _movetolocation) 0.0 99999.0) (.z _movetolocation)) false false))

(fn ConstructionScript)

(fn FindMovementLocation
  (if (== (Variables|/Game/Blueprints/Blueprints/BP_GameMode.BP_GameMode_C|GetNumPlayers (Variables|Default|GetGameMode)) 1)
    _
    (else
      _))
  (return (Transformation|GetActorLocation (Game|Player|GetPlayerPawn 0))))