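; BP_GameInfoInstance is a game info Blueprint that handles menu screens and hosting of multiplayer games.
; Menu and loading events lazily create and cache their widgets, add them to the viewport and set UI-only input, with the cursor shown for the main menu.
; Hosting shows the loading screen, sets up a session using player-count and LAN settings, then opens TestMap as a listen server.
; Session error handling remains a TODO.
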(event Custom|EV_ShowMainMenu
  (bind _returnvalue (Game|GetPlayerController 0))
  ;[1 1 1] Show Main Menu
  (Utilities|IsValid (Variables|Widgets|GetMainMenuRef)
    (:Is%20Valid
      _)
    (:Is%20Not%20Valid
      (bind _returnvalue_2 (UserInterface|CreateWidget "/Game/UI/WBP_MainMenu.WBP_MainMenu_C" _returnvalue))
      (Variables|Widgets|SetMainMenuRef _returnvalue_2)))
  (Input|SetInputModeUIOnly _returnvalue (Variables|Widgets|GetMainMenuRef) "DoNotLock")
  (UserInterface|Viewport|AddtoViewport (Variables|Widgets|GetMainMenuRef) 0)
  (Variables|/Script/Engine.PlayerController|SetbShowMouseCursor _returnvalue true))

(event Custom|EV_HostGame
  ;[1 1 1] Launch Online Session / TODO Set up Error Dialog
  (CallFunction|EVShowLoading)
  (|Session (Game|GetPlayerController 0) (Variables|ServerSettings|GetMaxPlayers) (Variables|ServerSettings|GetbEnableLan)
    (:then
      (Game|OpenLevel(byName) "TestMap" true "listen"))))

(event Custom|EV_ShowLoading
  (bind _returnvalue (Game|GetPlayerController 0))
  ;[1 1 1] Show Loading Screen
  (Utilities|IsValid (Variables|Widgets|GetLoadingRef)
    (:Is%20Valid
      _)
    (:Is%20Not%20Valid
      (bind _returnvalue_2 (UserInterface|CreateWidget "/Game/UI/WBP_Loading.WBP_Loading_C" _returnvalue))
      (Variables|Widgets|SetLoadingRef _returnvalue_2)))
  (Input|SetInputModeUIOnly _returnvalue (Variables|Widgets|GetLoadingRef) "DoNotLock")
  (UserInterface|Viewport|AddtoViewport (Variables|Widgets|GetLoadingRef) 0))