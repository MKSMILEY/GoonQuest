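; Shared follow camera that keeps the players from the game mode's player list in view.
; Each tick it averages their positions and traces down, settling on nearby ground when found.
; The largest distance reported by players linearly scales spring arm length between begin and end zoom thresholds.
; Zoom also raises the minimum X of the camera's clamped position, while Y stays non-negative.
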(event EventBeginPlay
  (bind _asbp_game_mode (Utilities|Casting|CastToBP_GameMode (Game|GetGameMode)))
  (bind _output_get (Variables|Default|SetGameMode _asbp_game_mode))
  (Variables|Default|SetPlayer%20List (Variables|/Game/Blueprints/BP_Gameplay/BP_GameMode.BP_GameMode_C|GetPlayerList _output_get)))

(event Collision|EventActorBeginOverlap
  (params (OtherActor :type Actor%20Object%20Reference)))

(event EventTick
  (params (DeltaSeconds :type Float%20%28single-precision%29))
  (bind (_zoommodifier _zoomxmodifer) (CallFunction|AdjustZoom))
  (Variables|/Script/Engine.SpringArmComponent|SetTargetArmLength (Variables|Default|GetSpringArm) (+ _zoommodifier (Variables|Default|GetDefaultSpringArmLength)))
  (bind _cameramovelocation (CallFunction|FindMovementLocation))
  (Transformation|SetActorLocation (Math|Vector|MakeVector (Math|Float|Clamp(Float) (.x _cameramovelocation) _zoomxmodifer 99999.0) (Math|Float|Clamp(Float) (.y _cameramovelocation) 0.0 99999.0) (.z _cameramovelocation)) false false))

(fn ConstructionScript)

(fn FindMovementLocation
  (bind _player_list (Variables|Default|GetPlayer%20List))
  (for _array_element _player_list
    (LocalVariables|SetSumVector (+ (Transformation|GetActorLocation _array_element) (LocalVariables|GetSumVector))))
  (bind _output_get (LocalVariables|SetCenterPosition (/ (LocalVariables|GetSumVector) (Utilities|Array|Length _player_list))))
  (bind (_outhit _returnvalue) (Collision|LineTraceByChannel (Math|Vector|MakeVector (.x _output_get) (.y _output_get) (.z _output_get)) (Math|Vector|MakeVector (.x _output_get) (.y _output_get) -1e+03) "TraceTypeQuery1" false (Variables|Default|GetPlayer%20List) "None"))
  (if (and _returnvalue (< (.Distance (Collision|BreakHitResult _outhit)) 4e+02))
    (return (.Location (Collision|BreakHitResult _outhit)))
    (elif (== (Utilities|Array|Length (Variables|Default|GetPlayer%20List)) 1)
      (return (Math|Vector|MakeVector (.x (LocalVariables|GetCenterPosition)) (.y (LocalVariables|GetCenterPosition)) (- (.z (LocalVariables|GetCenterPosition)) 97.0)))
      (else
        (return (LocalVariables|GetCenterPosition))))))

(fn AdjustZoom
  (for _array_element (Variables|Default|GetPlayer%20List)
    (if (> (Variables|/Game/Blueprints/BP_Characters/BP_PlayerCharacter/BP_Character.BP_Character_C|GetLargestDistance _array_element) (LocalVariables|GetMaxPlayerDistance))
      (LocalVariables|SetMaxPlayerDistance (Variables|/Game/Blueprints/BP_Characters/BP_PlayerCharacter/BP_Character.BP_Character_C|GetLargestDistance _array_element))))
  (if (> (LocalVariables|GetMaxPlayerDistance) (Variables|Default|GetBeginZoomDistance))
    (if (> (LocalVariables|GetMaxPlayerDistance) (Variables|Default|GetEndZoomDistance))
      (return (Variables|Default|GetMaxZoom) (Variables|Default|GetMaxZoomLocationAdjust))
      (else
        (return (* (Variables|Default|GetMaxZoom) (/ (- (LocalVariables|GetMaxPlayerDistance) (Variables|Default|GetBeginZoomDistance)) (- (Variables|Default|GetEndZoomDistance) (Variables|Default|GetBeginZoomDistance)))) (* (/ (- (LocalVariables|GetMaxPlayerDistance) (Variables|Default|GetBeginZoomDistance)) (- (Variables|Default|GetEndZoomDistance) (Variables|Default|GetBeginZoomDistance))) (Variables|Default|GetMaxZoomLocationAdjust)))))
    (else
      (return 0.0 0.0))))