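; BP_CharacterSelectVolume is a character select actor that displays the portrait of one character on its PaperSprite.
; Its EV_RetrieveInfo event casts player controller 0 to BP_PlayerController and reads the CharacterInfoList on its CharacterManagerRef.
; It caches the entry at CharacterNum in CharacterInfoRef and applies that entry's SPRPortrait to the sprite.
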(event Custom|EV_RetrieveInfo
  (bind _asbp_player_controller (Utilities|Casting|CastToBP_PlayerController (Game|GetPlayerController 0)))
  (bind _output_get (Variables|Default|SetCharacterInfoRef (Utilities|Array|Get(acopy) (Variables|/Game/Blueprints/BP_Characters/BP_CharacterManager.BP_CharacterManager_C|GetCharacterInfoList (Variables|/Game/Blueprints/BP_Characters/BP_PlayerCharacter/BP_PlayerController.BP_PlayerController_C|GetCharacterManagerRef _asbp_player_controller)) (Variables|Default|GetCharacterNum))))
  (Rendering|Components|Sprite|SetSprite (Variables|Default|GetPaperSprite) (Variables|/Game/Blueprints/BP_Characters/CharacterBPs/BP_CharacterInfo.BP_CharacterInfo_C|GetSPR_Portrait _output_get)))

(fn ConstructionScript
  (|CallParentFunction))