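; BP_InteractVolume is a trigger volume that shows a Prompt component while a player character stands inside it.
; Begin overlap reveals the prompt for any BP_PlayerCharacter and ignores other actors.
; End overlap hides it only when no player characters still overlap, so one player leaving does not clear it for another.
; It contains only this visibility logic, with no interaction input handling.
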(event Collision|EventActorBeginOverlap
  (params (OtherActor :type Actor%20Object%20Reference))
  (Utilities|Casting|CastToBP_PlayerCharacter OtherActor)
  (Rendering|SetVisibility (Variables|Default|GetPrompt) true false))

(event Collision|EventActorEndOverlap
  (params (OtherActor :type Actor%20Object%20Reference))
  (Utilities|Casting|CastToBP_PlayerCharacter OtherActor)
  (if (not (> (Utilities|Array|Length (Collision|GetOverlappingActors "/Game/Blueprints/BP_Characters/BP_PlayerCharacter/BP_PlayerCharacter.BP_PlayerCharacter_C" :!class /Script/Engine.Actor)) 0))
    (Rendering|SetVisibility (Variables|Default|GetPrompt) false false)))

(fn ConstructionScript)