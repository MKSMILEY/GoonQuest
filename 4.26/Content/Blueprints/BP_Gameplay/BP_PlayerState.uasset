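; Player state that holds a player's number, available character roster and character manager.
; On lobby init it caches the game instance and maps the unlock flags in PlayerInfo by index onto the instance's master character list to build that roster.
; A separate event constructs a BP_CharacterManager object owned by the player state, and the reference's RepNotify initializes it.
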(event Custom|EV_LobbyInit
  (params (PlayerNum :type Integer))
  (Variables|Default|SetPlayerNumber PlayerNum)
  (bind _asbp_game_info_instance (Utilities|Casting|CastToBP_GameInfoInstance (Game|GetGameInstance)))
  (bind _output_get (Variables|Default|SetGameInstanceRef _asbp_game_info_instance))
  (for (_array_element _array_index) (.unlockedcharacters (Variables|Default|GetPlayerInfo))
    (if _array_element
      (Utilities|Array|Add (Variables|Default|GetPlayerAvailableCharacters) (Utilities|Array|Get(acopy) (Variables|/Game/Blueprints/BP_Gameplay/BP_GameInfoInstance.BP_GameInfoInstance_C|GetAllAvailableCharacters _output_get) _array_index)))))

(event Custom|EV_CreateCharacterManager
  (bind _returnvalue (Game|ConstructObjectfromClass "/Game/Blueprints/BP_Characters/BP_CharacterManager.BP_CharacterManager_C" self))
  (Variables|Default|SetCharacterManagerRef _returnvalue))

(event EventBeginPlay)

(event EventTick
  (params (DeltaSeconds :type Float%20%28single-precision%29)))

(fn ConstructionScript)

(fn OnRepCharacterManagerRef
  (Default|EVInitialize (Variables|Default|GetCharacterManagerRef)))