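; BP_FollowCamera is a shared follow camera that keeps the player characters framed, updated only with authority.
; UpdatePlayers rebuilds the character list from the GameState's players.
; Each tick moves it to their average position, snapped to ground a downward trace finds nearby, with X and Y clamped.
; The largest player distance scales spring arm length and minimum X linearly between begin and end zoom thresholds.
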(event Custom|UpdatePlayers
  (Networking|SwitchHasAuthority
    (:Authority
      (Utilities|Array|Clear (Variables|Default|GetPlayerCharacterList))
      (for _array_element (Variables|/Game/Blueprints/BP_Gameplay/BP_GameState.BP_GameState_C|GetPlayerList (Variables|Default|GetGameStateRef))
        (bind _asbp_player_character (Utilities|Casting|CastToBP_PlayerCharacter (Pawn|GetControlledPawn _array_element)))
        (Utilities|Array|Add (Variables|Default|GetPlayerCharacterList) _asbp_player_character)))))

(event EventPossessed
  (params (NewController :type Controller%20Object%20Reference))
  (Networking|SwitchHasAuthority
    (:Authority
      (bind _asbp_game_mode (Utilities|Casting|CastToBP_GameMode (Game|GetGameMode)))
      (Variables|Default|SetGameModeRef _asbp_game_mode)
      (bind _asbp_game_state (Utilities|Casting|CastToBP_GameState (Game|GetGameState)))
      (Variables|Default|SetGameStateRef _asbp_game_state))))

(event EventTick
  (params (DeltaSeconds :type Float%20%28single-precision%29))
  (Networking|SwitchHasAuthority
    (:Authority
      (bind (_zoommodifier _zoomxmodifer) (CallFunction|AdjustZoom))
      (Variables|/Script/Engine.SpringArmComponent|SetTargetArmLength (Variables|Default|GetSpringArm) (+ _zoommodifier (Variables|Default|GetDefaultSpringArmLength)))
      (bind _cameramovelocation (CallFunction|FindMovementLocation))
      (Transformation|SetActorLocation (Math|Vector|MakeVector (Math|Float|Clamp(Float) (.x _cameramovelocation) _zoomxmodifer 99999.0) (Math|Float|Clamp(Float) (.y _cameramovelocation) 0.0 99999.0) (.z _cameramovelocation)) false false))))

(fn ConstructionScript)

(fn FindMovementLocation
  (bind _playercharacterlist (Variables|Default|GetPlayerCharacterList))
  (for _array_element (Variables|Default|GetPlayerCharacterList)
    (LocalVariables|SetSumVector (+ (Transformation|GetActorLocation _array_element) (LocalVariables|GetSumVector))))
  (bind _output_get (LocalVariables|SetCenterPosition (/ (LocalVariables|GetSumVector) (Utilities|Array|Length _playercharacterlist))))
  (bind (_outhit _returnvalue) (Collision|LineTraceByChannel (Math|Vector|MakeVector (.x _output_get) (.y _output_get) (.z _output_get)) (Math|Vector|MakeVector (.x _output_get) (.y _output_get) -1e+03) "TraceTypeQuery1" false _playercharacterlist "None"))
  (if (and _returnvalue (< (.Distance (Collision|BreakHitResult _outhit)) 4e+02))
    (return (.Location (Collision|BreakHitResult _outhit)))
    (elif (== (Utilities|Array|Length (Variables|Default|GetPlayerCharacterList)) 1)
      (return (Math|Vector|MakeVector (.x (LocalVariables|GetCenterPosition)) (.y (LocalVariables|GetCenterPosition)) (- (.z (LocalVariables|GetCenterPosition)) 97.0)))
      (else
        (return (LocalVariables|GetCenterPosition))))))

(fn AdjustZoom
  (for _array_element (Variables|Default|GetPlayerCharacterList)
    (if (> (Variables|/Game/Blueprints/BP_Characters/BP_PlayerCharacter/BP_PlayerCharacter.BP_PlayerCharacter_C|GetLargestDistance _array_element) (LocalVariables|GetMaxPlayerDistance))
      (LocalVariables|SetMaxPlayerDistance (Variables|/Game/Blueprints/BP_Characters/BP_PlayerCharacter/BP_PlayerCharacter.BP_PlayerCharacter_C|GetLargestDistance _array_element))))
  (if (> (LocalVariables|GetMaxPlayerDistance) (Variables|Default|GetBeginZoomDistance))
    (if (> (LocalVariables|GetMaxPlayerDistance) (Variables|Default|GetEndZoomDistance))
      (return (Variables|Default|GetMaxZoom) (Variables|Default|GetMaxZoomLocationAdjust))
      (else
        (return (* (Variables|Default|GetMaxZoom) (/ (- (LocalVariables|GetMaxPlayerDistance) (Variables|Default|GetBeginZoomDistance)) (- (Variables|Default|GetEndZoomDistance) (Variables|Default|GetBeginZoomDistance)))) (* (/ (- (LocalVariables|GetMaxPlayerDistance) (Variables|Default|GetBeginZoomDistance)) (- (Variables|Default|GetEndZoomDistance) (Variables|Default|GetBeginZoomDistance))) (Variables|Default|GetMaxZoomLocationAdjust)))))
    (else
      (return 0.0 0.0))))