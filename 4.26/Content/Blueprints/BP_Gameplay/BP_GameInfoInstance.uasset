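; BP_GameInfoInstance is the game instance that manages menu and loading widgets and the multiplayer session flow.
; WBP_MainMenu calls it to host a session, which opens L_TestMap as a listen server, or to join a found one.
; Main menu and loading widgets are created once and reused, and a separate event destroys the session.
; Network, travel and session failures route to DisplayErrorMessage, which is currently an empty stub.
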(event Custom|EV_ShowMainMenu
  (bind _returnvalue (Game|GetPlayerController 0))
  ;[1 1 1] Show Main Menu
  (Utilities|IsValid (Variables|Widgets|GetWBPMainMenu)
    (:Is%20Valid
      _)
    (:Is%20Not%20Valid
      (bind _returnvalue_2 (UserInterface|CreateWidget "/Game/UI/WBP_MainMenu.WBP_MainMenu_C" _returnvalue))
      (Variables|Widgets|SetWBPMainMenu _returnvalue_2)))
  (UserInterface|Viewport|AddtoViewport (Variables|Widgets|GetWBPMainMenu) 0)
  (Variables|/Script/Engine.PlayerController|SetbShowMouseCursor _returnvalue false))

(event Custom|EV_ShowLoading
  ;[1 1 1] Show Loading
  (Utilities|IsValid (Variables|Widgets|GetWBPLoading)
    (:Is%20Valid
      _)
    (:Is%20Not%20Valid
      (bind _returnvalue (UserInterface|CreateWidget "/Game/UI/WBP_Loading.WBP_Loading_C" (Game|GetPlayerController 0)))
      (Variables|Widgets|SetWBPLoading _returnvalue)))
  (UserInterface|Viewport|AddtoViewport (Variables|Widgets|GetWBPLoading) 0))

(event Custom|EV_LaunchLobby
  (params (NumberOfPlayers :type Integer) (bEnableLan :type Boolean) (ServerName :type Text))
  ;[1 1 1] Launch Lobby w/ Host Settings - Called in WBP_MainMenu
  (Variables|ServerSettings|SetNumPlayers NumberOfPlayers)
  (Variables|ServerSettings|SetServer%20Name ServerName)
  (CallFunction|EvShowLoading)
  (|Session (Game|GetPlayerController 0) (Variables|ServerSettings|GetNumPlayers) bEnableLan
    (:OnSuccess
      (Game|OpenLevel(byName) "L_TestMap" true "listen"))
    (:OnFailure
      (Utilities|DisplayErrorMessage "Failed to create session. Please try again."))))

(event Custom|EV_JoinServer
  (params (SessionToJoin :type Blueprint%20Session%20Result%20Structure))
  ;[1 1 1] Join Found Session - Called in WBP_MainMenu
  (CallFunction|EvShowLoading)
  (|JoinSession (Game|GetPlayerController 0) SessionToJoin
    (:OnFailure
      (Utilities|DisplayErrorMessage "Failed to join dession. Please try again."))))

(event Custom|EV_DestoySessionCaller
  (params (PlayerController :type Player%20Controller%20Object%20Reference))
  (|DestroySession PlayerController))

(event EventHandleNetworkError
  (params (FailureType :type ENetworkFailure%20Enum :default "NetDriverAlreadyExists") (bIsServer :type Boolean))
  (if bIsServer
    _
    (else
      _))
  (Utilities|DisplayErrorMessage (Utilities|String|EnumtoString FailureType)))

(event EventHandleTravelError
  (params (FailureType :type ETravelFailure%20Enum :default "NoLevel"))
  (Utilities|DisplayErrorMessage (Utilities|String|EnumtoString FailureType)))