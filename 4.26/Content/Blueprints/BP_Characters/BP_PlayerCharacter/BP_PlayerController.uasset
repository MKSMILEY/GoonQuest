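; Player controller that sets up character data, requests spawning and handles the character selection UI.
; On local BeginPlay it creates a character manager, then for each select volume retrieves info, shares the manager with GameState and sends a server RPC for GameMode to spawn the player.
; It shows or removes the selection widget, toggling input mode and cursor, and forwards character choices to the pawn's server RPC.
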(event Custom|DisplaySelectCharacterWidget
  (params (CharacterNumber :type Integer))
  (Utilities|IsValid (Variables|Default|GetWBP_SelectCharacterInfo)
    (:Is%20Valid
      _)
    (:Is%20Not%20Valid
      (bind _returnvalue (Game|ConstructObjectfromClass "/Game/UI/WBP_SelectCharacterInfo.WBP_SelectCharacterInfo_C" self))
      (Variables|Default|SetWBP_SelectCharacterInfo _returnvalue)))
  (Default|SetCharacter (Variables|Default|GetWBP_SelectCharacterInfo) (Utilities|Array|Get(acopy) (Variables|/Game/Blueprints/BP_Characters/BP_CharacterManager.BP_CharacterManager_C|GetCharacterInfoList (Variables|Default|GetCharacterManagerRef)) CharacterNumber))
  (Input|SetInputModeGameandUI self (Variables|Default|GetWBP_SelectCharacterInfo) "DoNotLock" false)
  (Variables|Default|SetbShowMouseCursor true)
  (UserInterface|Viewport|AddtoViewport (Variables|Default|GetWBP_SelectCharacterInfo) 0))

(event Custom|RemoveSelectCharacterWidget
  (Input|SetInputModeGameOnly self)
  (Variables|Default|SetbShowMouseCursor false)
  (Widget|RemovefromParent (Variables|Default|GetWBP_SelectCharacterInfo)))

(event Custom|UpdateCharacterInfo
  (params (CharacterNumber :type Integer))
  (bind _asbp_player_character (Utilities|Casting|CastToBP_PlayerCharacter (Pawn|GetControlledPawn)))
  (Default|RPCServerUpdateCharacterInfo _asbp_player_character CharacterNumber))

(event Custom|RPC_Server_SpawnPlayer
  (bind _asbp_game_mode (Utilities|Casting|CastToBP_GameMode (Game|GetGameMode)))
  (Default|EVSpawnCharacter _asbp_game_mode self))

(event EventBeginPlay
  (if (Pawn|IsLocalPlayerController)
    (Utilities|IsValid (Variables|Default|GetCharacterManagerRef)
      (:Is%20Valid
        _)
      (:Is%20Not%20Valid
        (CallFunction|CreateCharacterManager)))
    (bind _outactors (Actor|GetAllActorsOfClass "/Game/Blueprints/BP_Gameplay/Volumes/BP_CharacterSelectVolume.BP_CharacterSelectVolume_C"))
    (for _array_element _outactors
      (Default|EVRetrieveInfo _array_element)
      (bind _asbp_game_state (Utilities|Casting|CastToBP_GameState (Game|GetGameState)))
      (Variables|/Game/Blueprints/BP_Gameplay/BP_GameState.BP_GameState_C|SetCharacterManagerRef _asbp_game_state (Variables|Default|GetCharacterManagerRef))
      (CallFunction|RPCServerSpawnPlayer))))

(fn ConstructionScript)

(fn CreateCharacterManager
  (bind _returnvalue (Game|ConstructObjectfromClass "/Game/Blueprints/BP_Characters/BP_CharacterManager.BP_CharacterManager_C" self))
  (bind _output_get (Variables|Default|SetCharacterManagerRef _returnvalue))
  (Default|EVInitialize _output_get))

(fn RetrieveCharacter
  (params (CharacterNumber :type Integer))
  (return (Utilities|Array|Get(acopy) (Variables|/Game/Blueprints/BP_Characters/BP_CharacterManager.BP_CharacterManager_C|GetCharacterInfoList (Variables|Default|GetCharacterManagerRef)) CharacterNumber)))