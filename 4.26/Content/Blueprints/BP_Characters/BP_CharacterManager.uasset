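; BP_CharacterManager creates and holds the game's character info objects.
; EV_Initialize constructs five BP_CharacterInfo objects, each of its own class with the manager as outer, skipping any slot that is already valid.
; Each new object is stored in its own variable and added to CharacterInfoList.
; A final loop sets every listed character's ExperiencePoints to the same fixed value, overwriting existing values on each initialization.
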(event Custom|EV_Initialize
  (Utilities|FlowControl|Sequence
    (:then_0
      (Utilities|IsValid (Variables|Default|GetCharacterInfo1)
        (:Is%20Not%20Valid
          (bind _returnvalue (Game|ConstructObjectfromClass "/Game/Blueprints/BP_Characters/CharacterBPs/BP_CharacterInfo01.BP_CharacterInfo01_C" self))
          (bind _output_get (Variables|Default|SetCharacterInfo1 _returnvalue))
          (Utilities|Array|Add (Variables|Default|GetCharacterInfoList) _output_get))))
    (:then_1
      (Utilities|IsValid (Variables|Default|GetCharacterInfo2)
        (:Is%20Not%20Valid
          (bind _returnvalue_2 (Game|ConstructObjectfromClass "/Game/Blueprints/BP_Characters/CharacterBPs/BP_CharacterInfo02.BP_CharacterInfo02_C" self))
          (bind _output_get_2 (Variables|Default|SetCharacterInfo2 _returnvalue_2))
          (Utilities|Array|Add (Variables|Default|GetCharacterInfoList) _output_get_2))))
    (:then_2
      (Utilities|IsValid (Variables|Default|GetCharacterInfo3)
        (:Is%20Not%20Valid
          (bind _returnvalue_3 (Game|ConstructObjectfromClass "/Game/Blueprints/BP_Characters/CharacterBPs/BP_CharacterInfo03.BP_CharacterInfo03_C" self))
          (bind _output_get_3 (Variables|Default|SetCharacterInfo3 _returnvalue_3))
          (Utilities|Array|Add (Variables|Default|GetCharacterInfoList) _output_get_3))))
    (:then_3
      (Utilities|IsValid (Variables|Default|GetCharacterInfo4)
        (:Is%20Not%20Valid
          (bind _returnvalue_4 (Game|ConstructObjectfromClass "/Game/Blueprints/BP_Characters/CharacterBPs/BP_CharacterInfo04.BP_CharacterInfo04_C" self))
          (bind _output_get_4 (Variables|Default|SetCharacterInfo4 _returnvalue_4))
          (Utilities|Array|Add (Variables|Default|GetCharacterInfoList) _output_get_4))))
    (:then_4
      (Utilities|IsValid (Variables|Default|GetCharacterInfo5)
        (:Is%20Not%20Valid
          (bind _returnvalue_5 (Game|ConstructObjectfromClass "/Game/Blueprints/BP_Characters/CharacterBPs/BP_CharacterInfo05.BP_CharacterInfo05_C" self))
          (bind _output_get_5 (Variables|Default|SetCharacterInfo5 _returnvalue_5))
          (Utilities|Array|Add (Variables|Default|GetCharacterInfoList) _output_get_5))))
    (:then_5
      (for _array_element (Variables|Default|GetCharacterInfoList)
        (Variables|/Game/Blueprints/BP_Characters/CharacterBPs/BP_CharacterInfo.BP_CharacterInfo_C|SetExperiencePoints _array_element 1000)))))